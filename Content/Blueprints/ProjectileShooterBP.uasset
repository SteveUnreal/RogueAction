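; ProjectileShooterBP is a turret-style actor that tracks the player and launches projectiles.
; Every tick it rotates to face the first player's pawn, using GetNewRotation to build a rotation from the direction between them.
; BeginPlay calls FireProjectile to start a looping two-second timer, apparently driving FireAway, which spawns a MagicProjectileBP at the actor's location aimed at that pawn.
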(event `self.ReceiveBeginPlay`
  (`self.FireProjectile`))

(event `self.ReceiveTick`
  (params (DeltaSeconds :type "Float (single-precision)"))
  (bind _resultrotation (`self.GetNewRotation`))
  (`self.K2_SetActorRotation` _resultrotation))

(event `FireAway`
  (bind _resultrotation (`self.GetNewRotation`))
  (`|SpawnActorFromClass` "/Game/Blueprints/MagicProjectileBP.MagicProjectileBP_C" (`KismetMathLibrary.MakeTransform` (`self.K2_GetActorLocation`) _resultrotation) "Undefined" "OverrideRootScale" null null))

(fn `FireProjectile`
  (`KismetSystemLibrary.K2_SetTimerDelegate` (`|CreateDelegate` :!event `FireAway`) 2.0 true))

(fn `GetNewRotation`
  (returns (ResultRotation :type "Rotator Structure"))
  (return (`KismetMathLibrary.MakeRotFromX` (- (`self.K2_GetActorLocation` (`GameplayStatics.GetPlayerPawn` 0)) (`self.K2_GetActorLocation`)))))

(fn `UserConstructionScript`)