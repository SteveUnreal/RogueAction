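; BP_Lever is an interactable lever actor that toggles between on and off when a pawn interacts with it.
; Interact flips IsOn and snaps the handle mesh to an opposite pitch for each state, without animation.
; Either way, it forwards an interact message with the instigating pawn to SelectedActor, so the lever can trigger another actor.
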(event `SGameplayInterface.Interact`
  (params (InstigatorPawn :type "Actor Object Reference"))
  (bind _selectedactor (`self.SelectedActor`))
  (bind _handlemesh (`self.HandleMesh`))
  (if (`self.IsOn`)
    (`SceneComponent.K2_SetRelativeRotation` _handlemesh (`KismetMathLibrary.MakeRotator` 0.0 25.0) false false)
    (set `self.IsOn` false)
    (message `SGameplayInterface.Interact` _selectedactor InstigatorPawn)
    (else
      (`SceneComponent.K2_SetRelativeRotation` _handlemesh (`KismetMathLibrary.MakeRotator` 0.0 -25.0) false false)
      (set `self.IsOn` true)
      (message `SGameplayInterface.Interact` _selectedactor InstigatorPawn))))

(fn `UserConstructionScript`)